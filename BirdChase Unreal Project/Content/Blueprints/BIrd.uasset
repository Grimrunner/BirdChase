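; Player-controlled flying bird that collects coins for score and ends the game on hitting a dragon, then restarts the level.
; Roll, pitch and yaw inputs drive paired thrust components for rotation.
; Tick integrates throttle and brake into a clamped Acceleration value that moves the actor along its local Y axis.
; That value also scales camera FOV between set limits, while a scene capture keeps a fixed top-down world rotation.
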(event EventTick
  (params (DeltaSeconds :type Float%20%28single-precision%29))
  ;[1 1 1] Updates
  (Utilities|FlowControl|Sequence
    (:then_0
      ;[1 1 1] Update Acceleration
      (if (> (Input|AxisValues|GetBrake) 0.0)
        (Variables|Default|SetAcceleration (- (Variables|Default|GetAcceleration) (* (Variables|Default|GetBrakeSpeed) DeltaSeconds)))
        (elif (> (Input|AxisValues|GetEngineThrust) 0.0)
          (Variables|Default|SetAcceleration (+ (Variables|Default|GetAcceleration) (* (Variables|Default|GetAccelerationSpeed) DeltaSeconds)))
          (else
            (Variables|Default|SetAcceleration (- (Variables|Default|GetAcceleration) (* (Variables|Default|GetSlowdownSpeed) DeltaSeconds))))))
      (if (< (Variables|Default|GetAcceleration) 0.0)
        (Variables|Default|SetAcceleration 0.0)
        (elif (> (Variables|Default|GetAcceleration) (Variables|Default|GetMaxAcceleration))
          (Variables|Default|SetAcceleration (Variables|Default|GetMaxAcceleration))))
      (Transformation|AddActorLocalOffset (* "0,1.000000, 0" (* (* DeltaSeconds (Variables|Default|GetAcceleration)) (Variables|Default|GetSpeed))) false false))
    (:then_1
      ;[1 1 1] Update camera
      (CallFunction|CameraUpdate))
    (:then_2
      ;[1 1 1] Update rotation top-down camera
      (Transformation|SetWorldRotation (Variables|Default|GetSceneCaptureComponent2D) "-80.000000,90.000000,0.000000" false false))))

(event Collision|EventHit
  (params (MyComp :type Primitive%20Component%20Object%20Reference) (Other :type Actor%20Object%20Reference) (OtherComp :type Primitive%20Component%20Object%20Reference) (bSelfMoved :type Boolean) (HitLocation :type Vector :default "0, 0, 0") (HitNormal :type Vector :default "0, 0, 0") (NormalImpulse :type Vector :default "0, 0, 0") (Hit :type Hit%20Result%20Structure%20%28by%20ref%29))
  ;[1 1 1] Collide with dragon
  (Utilities|Casting|CastToDragon Other)
  (bind _asbp_hud (Utilities|Casting|CastToBP_HUD (HUD|GetHUD (Game|GetPlayerController 0))))
  (Default|DrawGameOver _asbp_hud)
  (Utilities|FlowControl|Delay 3.0)
  (bind _returnvalue (Game|GetCurrentLevelName true))
  (Game|OpenLevel(byName) (Utilities|String|StringToName _returnvalue)))

(event Collision|EventActorBeginOverlap
  (params (OtherActor :type Actor%20Object%20Reference))
  ;[1 1 1] Grabbing coins
  (Utilities|FlowControl|Sequence
    (:then_0
      (bind _ascoin (Utilities|Casting|CastToCoin OtherActor))
      (Actor|DestroyActor _ascoin)
      (Variables|Default|SetScore (+ (Variables|Default|GetScore) 1)))))

(event EventBeginPlay)

(event Input|ActionEvents|InputActionReset
  (params (Key :type Key%20Structure))
  ;[1 1 1] Reset level
  (:Pressed
    (bind _returnvalue (Game|GetCurrentLevelName true))
    (Game|OpenLevel(byName) (Utilities|String|StringToName _returnvalue))))

(event Input|AxisEvents|InputAxisRoll
  (params (AxisValue :type Float%20%28single-precision%29))
  (bind _rollstrength (Variables|Default|GetRollStrength))
  (bind _leftwingrollthrust (Variables|Default|GetLeftWingRollThrust))
  (bind _rightwingrollthrust (Variables|Default|GetRightWingRollThrust))
  (bind _returnvalue (* AxisValue _rollstrength))
  ;[1 1 1] Roll
  (if (== AxisValue 0.0)
    (Components|Activation|Deactivate _leftwingrollthrust)
    (Components|Activation|Deactivate _rightwingrollthrust)
    (else
      (Components|Activation|Activate _leftwingrollthrust false)
      (Variables|/Script/Engine.PhysicsThrusterComponent|SetThrustStrength _leftwingrollthrust _returnvalue)
      (Components|Activation|Activate _rightwingrollthrust false)
      (Variables|/Script/Engine.PhysicsThrusterComponent|SetThrustStrength _rightwingrollthrust _returnvalue))))

(event Input|AxisEvents|InputAxisPitch
  (params (AxisValue :type Float%20%28single-precision%29))
  (bind _pitchstrength (Variables|Default|GetPitchStrength))
  (bind _nosepitchthrust (Variables|Default|GetNosePitchThrust))
  (bind _tailpitchthrust (Variables|Default|GetTailPitchThrust))
  (bind _returnvalue (* AxisValue _pitchstrength))
  ;[1 1 1] Pitch
  (if (== AxisValue 0.0)
    (Components|Activation|Deactivate _tailpitchthrust)
    (Components|Activation|Deactivate _nosepitchthrust)
    (else
      (Components|Activation|Activate _tailpitchthrust false)
      (Variables|/Script/Engine.PhysicsThrusterComponent|SetThrustStrength _tailpitchthrust _returnvalue)
      (Components|Activation|Activate _nosepitchthrust false)
      (Variables|/Script/Engine.PhysicsThrusterComponent|SetThrustStrength _nosepitchthrust _returnvalue))))

(event Input|AxisEvents|InputAxisYaw
  (params (AxisValue :type Float%20%28single-precision%29))
  (bind _yawstrength (Variables|Default|GetYawStrength))
  (bind _tailyawthrust (Variables|Default|GetTailYawThrust))
  (bind _noseyawthrust (Variables|Default|GetNoseYawThrust))
  (bind _returnvalue (* AxisValue _yawstrength))
  ;[1 1 1] Yaw
  (if (== AxisValue 0.0)
    (Components|Activation|Deactivate _tailyawthrust)
    (Components|Activation|Deactivate _noseyawthrust)
    (else
      (Components|Activation|Activate _tailyawthrust false)
      (Variables|/Script/Engine.PhysicsThrusterComponent|SetThrustStrength _tailyawthrust _returnvalue)
      (Components|Activation|Activate _noseyawthrust false)
      (Variables|/Script/Engine.PhysicsThrusterComponent|SetThrustStrength _noseyawthrust _returnvalue))))

(fn ConstructionScript)

(fn CameraUpdate
  (bind _fovspeedminimum (Variables|Default|GetFovSpeedMinimum))
  (bind _acceleration (Variables|Default|GetAcceleration))
  (bind _fovminimum (Variables|Default|GetFovMinimum))
  ;[1 1 1] Update the field of view depending on speed
  (if (<= _acceleration _fovspeedminimum)
    (Camera|SetFieldOfView (Variables|Default|GetCamera) (Variables|Default|GetFovMinimum))
    (elif (>= _acceleration (Variables|Default|GetFovSpeedMaximum))
      (Camera|SetFieldOfView (Variables|Default|GetCamera) (Variables|Default|GetFovMaximum))
      (else
        (Camera|SetFieldOfView (Variables|Default|GetCamera) (+ (* (/ (- (Variables|Default|GetAcceleration) _fovspeedminimum) (- (Variables|Default|GetFovSpeedMaximum) (Variables|Default|GetFovSpeedMinimum))) (- (Variables|Default|GetFovMaximum) _fovminimum)) _fovminimum))))))