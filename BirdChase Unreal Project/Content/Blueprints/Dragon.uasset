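; Dragon actor that chases the player's Bird pawn, updated every tick.
; It smoothly interpolates its rotation toward the bird and measures the angle between its forward vector and the bird.
; That angle drives a clamped acceleration factor, gaining more the better it is aligned and slowing when the bird is outside a forward cone.
; The factor scales max speed for an unswept local forward move.
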(event EventTick
  (params (DeltaSeconds :type Float%20%28single-precision%29))
  ;[1 1 1] Updates
  (Utilities|FlowControl|Sequence
    (:then_0
      ;[1 1 1] Rotate towards the bird
      (bind _asbird (Utilities|Casting|CastToBird (Game|Player|GetPlayerPawn 0)))
      (Transformation|SetWorldRotation (Variables|Default|GetDragon) (Math|Interpolation|RInterpTo (Transformation|GetActorRotation) (Math|Rotator|FindLookatRotation (Transformation|GetActorLocation) (Transformation|GetActorLocation _asbird)) DeltaSeconds (Variables|Default|GetTurnSpeed)) false false)
      (Variables|Default|SetBirdAngle (Class|KismetMathLibrary|DegAcos (Math|Vector|DotProduct (Math|Vector|Normalize (Math|Vector|GetForwardVector (Variables|Default|GetDragon))) (Math|Vector|Normalize (- (Transformation|GetActorLocation _asbird) (Transformation|GetActorLocation)))))))
    (:then_1
      ;[1 1 1] Calculate acceleration
      (if (> (Variables|Default|GetBirdAngle) 45.0)
        (bind _output_get (Variables|Default|SetAcceleration (- (Variables|Default|GetAcceleration) (* (Variables|Default|GetDeaccelerationSpeed) DeltaSeconds))))
        (if (< _output_get 0.0)
          (Variables|Default|SetAcceleration 0.0))
        (else
          (bind _output_get_2 (Variables|Default|SetAcceleration (+ (Variables|Default|GetAcceleration) (* (* DeltaSeconds (Variables|Default|GetAccelerationSpeed)) (+ (/ (Variables|Default|GetBirdAngle) -45.0) 1.0)))))
          (if (> _output_get_2 1.0)
            (Variables|Default|SetAcceleration 1.0)))))
    (:then_2
      ;[1 1 1] Move
      (Transformation|AddActorLocalOffset (* "1.000000,0.000000, 0" (* (* DeltaSeconds 1e+02) (* (Variables|Default|GetMaxSpeed) (Variables|Default|GetAcceleration)))) false false))))

(fn ConstructionScript)